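; Test AI controller that runs BT_TestAI on possession and stores the possessed pawn as SelfActor in its blackboard.
; AI Perception updates for a sensed player-controlled pawn cancel the forget timer and set HasLineOfSight and TargetActor.
; Any other pawn update, including lost sight or a non-player pawn, starts a LineOfSightTimer delay that then clears both keys.
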(event OnTargetPerceptionUpdated(AI_Perception)
  (params (Actor :type Actor%20Object%20Reference) (Stimulus :type AI%20Stimulus%20Structure))
  (bind _blackboard (Variables|Default|GetBlackboard))
  (bind _aspawn (Utilities|Casting|CastToPawn Actor))
  (if (and (Class|Controller|IsPlayerController (Pawn|GetController _aspawn)) (.bSuccessfullySensed (Utilities|Struct|BreakAIStimulus Stimulus)))
    (Utilities|Time|ClearandInvalidateTimerbyHandle (Variables|Default|GetAITimer))
    (AI|Components|Blackboard|SetValueasBool _blackboard (Variables|Default|GetHasLineOfSight) true)
    (AI|Components|Blackboard|SetValueasObject _blackboard (Variables|Default|GetTargetActor) Actor)
    (else
      (bind _returnvalue (Utilities|Time|SetTimerbyEvent (delegate Custom|StartEnemyTimer) (Variables|Default|GetLineOfSightTimer)))
      (Variables|Default|SetAITimer _returnvalue))))

(event Custom|StartEnemyTimer
  (bind _blackboard (Variables|Default|GetBlackboard))
  (AI|Components|Blackboard|SetValueasBool _blackboard (Variables|Default|GetHasLineOfSight) false)
  (AI|Components|Blackboard|SetValueasObject _blackboard (Variables|Default|GetTargetActor) 0))

(event EventBeginPlay)

(event EventTick
  (params (DeltaSeconds :type Float%20%28single-precision%29)))

(event EventPossess
  (params (PossessedPawn :type Pawn%20Object%20Reference))
  (AI|RunBehaviorTree "/Game/AI/Test/BT_TestAI.BT_TestAI")
  (AI|Components|Blackboard|SetValueasObject (Variables|Default|GetBlackboard) (Variables|Default|GetSelfActor) PossessedPawn))

(fn ConstructionScript)